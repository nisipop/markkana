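; A coin spawner spot that drops physics-simulated coins from its location at randomized intervals, optionally stopping after a set time.
; A looping timer triggers a random delay, then spawns a StaticMeshActor with random rotation and configurable mesh, scale and mass.
; Each coin is stored with its spawn time, and a once-per-second timer destroys those past their lifespan, removing their array entries after the loop; zero lifespan keeps them.
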(event `CleanOldCoins`
  ;[1 1 1] Run clean coins every second
  (`KismetSystemLibrary.K2_SetTimerDelegate` (delegate `CallDeleteItemInArray`) 1.0 true))

(event `StopCoinCabacabana`
  ;[1 1 1] Stop spawn
  (if (`KismetSystemLibrary.K2_IsValidTimerHandle` (`self.CoinSpawnerEvent`))
    (`KismetSystemLibrary.K2_ClearAndInvalidateTimerHandle` (`self.CoinSpawnerEvent`))))

(event `CallDeleteItemInArray`
  ;[1 1 1] Run clean coins every second
  (`self.Handle Destruct Coin from Array` (`self.SpawnedCoinCollection`) (`self.CoinLifeSpanInSeconds`)))

(event `StartCoinCabacabana`
  ;[1 1 1] Spawn coins in given intervals
  (bind _returnvalue (`KismetSystemLibrary.K2_SetTimerDelegate` (delegate `SpawnCoin`) (`self.MinSpawnTime`) true true))
  (set `self.CoinSpawnerEvent` _returnvalue))

(event `self.ReceiveBeginPlay`
  (`|ExecutionSequence`
    (:`then_0`
      (`self.StartCoinCabacabana`))
    (:`then_1`
      (`self.CleanOldCoins`))
    (:`then_2`
      (if (> (`self.StopSpawnAfterSeconds`) 0)
        (`KismetSystemLibrary.Delay` (`KismetMathLibrary.Conv_Int64ToDouble` (`self.StopSpawnAfterSeconds`)))
        (`self.StopCoinCabacabana`)))))

(event `SpawnCoin`
  (bind _returnvalue (`KismetMathLibrary.RandomFloatInRange` 0.0 180.0))
  (bind _staticmeshcomponent (`StaticMeshActor.StaticMeshComponent` (`self.SpawnedCoinTemp`)))
  ;[1 1 1] Spawn coins in given intervals
  (`KismetSystemLibrary.Delay` (`KismetMathLibrary.RandomFloatInRange` (`self.MinSpawnTime`) (`self.MaxSpawnTime`)))
  (bind _returnvalue_2 (`|SpawnActorFromClass` "/Script/Engine.StaticMeshActor" (`KismetMathLibrary.MakeTransform` (`SceneComponent.K2_GetComponentLocation` (`self.DefaultSceneRoot`)) (`KismetMathLibrary.MakeRotator` _returnvalue _returnvalue _returnvalue) (`KismetMathLibrary.Conv_DoubleToVector` (`self.CoinScaleFactor`))) "Undefined" "MultiplyWithRoot" null null))
  (bind _output_get (set `self.SpawnedCoinTemp` _returnvalue_2))
  (`KismetArrayLibrary.Array_Add` (`self.SpawnedCoinCollection`) (make `/Game/MyBlueprints/S_CoinItemContainer` _output_get (`GameplayStatics.GetRealTimeSeconds`)))
  (`|ExecutionSequence`
    (:`then_0`
      (`SceneComponent.SetMobility` _staticmeshcomponent "Movable")
      (`StaticMeshComponent.SetStaticMesh` _staticmeshcomponent (`self.CoinMesh`)))
    (:`then_1`
      (`PrimitiveComponent.SetCollisionObjectType` _staticmeshcomponent "ECC_WorldDynamic"))
    (:`then_2`
      (`PrimitiveComponent.SetCollisionEnabled` (`StaticMeshActor.StaticMeshComponent` (`self.SpawnedCoinTemp`)) "QueryAndPhysics"))
    (:`then_3`
      (`PrimitiveComponent.SetSimulatePhysics` (`StaticMeshActor.StaticMeshComponent` (`self.SpawnedCoinTemp`)) true))
    (:`then_4`
      (`PrimitiveComponent.SetMassOverrideInKg` (`StaticMeshActor.StaticMeshComponent` (`self.SpawnedCoinTemp`)) "None" (`self.CoinWeight`) true))))

(fn `Handle Destruct Coin from Array`
  (params (CoinItems :type "Array of /Game/MyBlueprints/S_CoinItemContainer Structure") (CoinLifeSpan :type "Float (double-precision)" :default 30.0))
  ;[1 1 1] Destroy coin reference in array based on given coin life span
  (if (and (> CoinLifeSpan 0.0) (== (`self.IsCleaningCoins`) false))
    (set `self.IsCleaningCoins` true)
    (`KismetArrayLibrary.Array_Clear` (`self.ObsoleteIndexes`))
    (for (_array_element _array_index) CoinItems
      (`/Engine/EditorBlueprintResources/StandardMacros.IsValid` (break `/Game/MyBlueprints/S_CoinItemContainer` _array_element)
        (:`Is Valid`
          (if (> (- (`GameplayStatics.GetRealTimeSeconds`) (`.CreatedRealTimeSeconds_7_306618A8426CF6E3DDEA72A72ED4E138` (break `/Game/MyBlueprints/S_CoinItemContainer` _array_element))) CoinLifeSpan)
            (`self.K2_DestroyActor` (break `/Game/MyBlueprints/S_CoinItemContainer` _array_element))
            (`KismetArrayLibrary.Array_Add` (`self.ObsoleteIndexes`) _array_index)))))
    ;[1 1 1] Clean the original array after loop
    (for (_ _array_index_2) (`self.ObsoleteIndexes`)
      (`KismetArrayLibrary.Array_Remove` (`self.SpawnedCoinCollection`) _array_index_2))
    (set `self.IsCleaningCoins` false)))

(fn `UserConstructionScript`)