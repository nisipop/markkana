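; Radial force actor that fires physics impulses on a repeating timer.
; The construction script copies the actor's radius and strength variables onto its RadialForce component.
; On BeginPlay a looping timer gets a random interval between the min and max pulse times, picked once, and calls FireImpulse on each tick of that timer.
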(event `self.ReceiveBeginPlay`
  (`KismetSystemLibrary.K2_SetTimerDelegate` (delegate `ImpulseFire`) (`KismetMathLibrary.RandomFloatInRange` (`self.MinPulseTime`) (`self.MaxPulseTime`)) true))

(event `ImpulseFire`
  (`RadialForceComponent.FireImpulse` (`self.RadialForce`)))

(fn `UserConstructionScript`
  (bind _radialforce (`self.RadialForce`))
  (set `RadialForceComponent.Radius` (`self.ImpulseRadius`) _radialforce)
  (set `RadialForceComponent.ImpulseStrength` (`self.ImpulseStrength`) _radialforce))